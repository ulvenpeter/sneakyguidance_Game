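; Construction-script tool actor that converts static mesh components across the level into instanced static meshes.
; It gathers components from all actors, filtering by ignore tags and class names, then hides the originals.
; It groups them by mesh name and materials, creating one instanced component per group with instances at the original world transforms.
; ConvertToInst triggers a fresh collection, while EditMode makes the original meshes visible again for editing.
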(event EventBeginPlay)

(event EventActorBeginOverlap
  (params (OtherActor :type Actor%20Object%20Reference)))

(event EventTick
  (params (DeltaSeconds :type Float%20%28single-precision%29)))

(fn ConstructionScript
  (if (Variables|Default|GetConvertToInst)
    (Variables|Setup|SetEditMode false :!label _label)
    (CallFunction|CollectComponents) ; Collect all the components that we need to convert to instances
    ;[1 1 1] Instances info clearing
    (Utilities|Array|Clear (Variables|Default|GetinstanceConf))
    (CallFunction|ChangeVisibility false) ; Disable original static mesh components
    (CallFunction|AddInst :!label _label_2) ; Place instanced meshes
    (Variables|Default|SetConvertedToInst true)
    (Variables|Default|SetConvertToInst false)
    (elif (Variables|Setup|GetEditMode)
      (CallFunction|ChangeVisibility true) ; Enable original meshes
      (Variables|Default|SetConvertedToInst false)
      (elif (Variables|Default|GetConvertedToInst)
        (goto _label_2)
        (else
          (goto _label))))))

(fn AddInst
  (for _array_element (Variables|notUsable|Getcompinents)
    (Utilities|Array|Clear (LocalVariables|GettmpMats))
    (for _index (range 0 (Rendering|Material|GetNumMaterials _array_element))
      (Utilities|Array|Add (LocalVariables|GettmpMats) (Rendering|Material|GetMaterial _array_element _index)))
    (Utilities|Array|Clear (LocalVariables|GettransformArray))
    (LocalVariables|Setfinded false)
    (bind (_array_element_2 _array_index) (Utilities|Array|ForEachLoopwithBreak (Variables|Default|GetinstanceConf))
      (:LoopBody
        (bind _equal (CallFunction|CheckMats (.materials (Utilities|Struct|BreakSTRUCT_InstacedMeshesInfo _array_element_2)) (LocalVariables|GettmpMats)))
        (if (and _equal (Utilities|Enum|Equal(Enum) (Utilities|GetDisplayName (Variables|/Script/Engine.StaticMeshComponent|GetStaticMesh _array_element)) (Utilities|GetDisplayName (.mesh (Utilities|Struct|BreakSTRUCT_InstacedMeshesInfo _array_element_2)))))
          (bind _output_get (LocalVariables|SettransformArray (.location (Utilities|Struct|BreakSTRUCT_InstacedMeshesInfo _array_element_2))))
          (Utilities|Array|Add _output_get (Transformation|GetWorldTransform _array_element))
          (LocalVariables|Setfinded true)
          (Utilities|Array|SetArrayElem (Variables|Default|GetinstanceConf) _array_index (Utilities|Struct|MakeSTRUCT_InstacedMeshesInfo :mesh (.mesh (Utilities|Struct|BreakSTRUCT_InstacedMeshesInfo _array_element_2)) :location (LocalVariables|GettransformArray) :materials (LocalVariables|GettmpMats)))))
      (:Completed
        (if (not (LocalVariables|Getfinded))
          (Utilities|Array|Add (Variables|Default|GetinstanceConf) (Utilities|Struct|MakeSTRUCT_InstacedMeshesInfo :mesh (Variables|/Script/Engine.StaticMeshComponent|GetStaticMesh _array_element) :location (Utilities|Array|MakeArray (Transformation|GetWorldTransform _array_element)) :materials (LocalVariables|GettmpMats)))))))
  (CallFunction|PlaceInst))

(fn ChangeVisibility
  (params (bNewVisibility :type Boolean))
  (for _array_element (Variables|notUsable|Getcompinents)
    (Rendering|SetVisibility _array_element bNewVisibility false))
  (return))

(fn PlaceInst
  (for _array_element (Variables|Default|GetinstanceConf)
    (bind _returnvalue (AddComponent|AddInstancedStaticMeshComponent false))
    (bind _returnvalue_2 (Components|StaticMesh|SetStaticMesh _returnvalue (.mesh (Utilities|Struct|BreakSTRUCT_InstacedMeshesInfo _array_element))))
    (for (_array_element_2 _array_index) (.materials (Utilities|Struct|BreakSTRUCT_InstacedMeshesInfo _array_element))
      (Rendering|Material|SetMaterial _returnvalue _array_index _array_element_2))
    (if _returnvalue_2
      (for _array_element_3 (.location (Utilities|Struct|BreakSTRUCT_InstacedMeshesInfo _array_element))
        (Components|InstancedStaticMesh|AddInstance _returnvalue _array_element_3)))))

(fn CollectComponents
  (Utilities|Array|Clear (Variables|notUsable|Getcompinents))
  (Utilities|Array|Clear (Variables|Default|Getactors))
  (bind _outactors (Actor|GetAllActorsOfClass "/Script/Engine.Actor"))
  (bind _output_get (Variables|Default|Setactors _outactors))
  (for _array_element _output_get
    (bind _returnvalue (CallFunction|CheckTags (Variables|/Script/Engine.Actor|GetTags _array_element)))
    (if (and _returnvalue (Utilities|ExcludeClasess (Utilities|GetClassDisplayName (Utilities|GetClass _array_element))))
      (for _array_element_2 (Actor|GetComponentsByClass _array_element "/Script/Engine.StaticMeshComponent")
        (bind _returnvalue_2 (CallFunction|CheckTags (Variables|/Script/Engine.ActorComponent|GetComponentTags _array_element_2)))
        (if (and _returnvalue_2 (Utilities|ExcludeClasess (Utilities|GetClassDisplayName (Utilities|GetClass _array_element_2))))
          (Utilities|Array|Add (Variables|notUsable|Getcompinents) _array_element_2)))))
  (return))

(fn CheckTags
  (params (TargetArray :type Array%20of%20Names))
  (bind _array_element (Utilities|Array|ForEachLoopwithBreak (Variables|Setup|GetignoreTags) :!label _label)
    (:LoopBody
      (bind _output_get (LocalVariables|SettmpB (< (Utilities|Array|FindItem TargetArray _array_element) 0)))
      (if (not _output_get)
        (goto _label Break)))
    (:Completed
      (return (LocalVariables|GettmpB)))))

(fn CheckMats
  (params (oldVal :type Array%20of%20Material%20Interface%20Object%20References) (newVal :type Array%20of%20Material%20Interface%20Object%20References))
  (if (!= (Utilities|Array|Length oldVal) (Utilities|Array|Length newVal))
    (LocalVariables|SetequalMAt false)
    (else
      (for _array_element oldVal
        (if (< (Utilities|Array|FindItem newVal _array_element) 0)
          (LocalVariables|SetequalMAt false)))))
  (return (LocalVariables|GetequalMAt)))