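; Growing-vines actor that reveals two animated skeletal vine meshes when the player character reaches it.
; Both meshes start hidden on BeginPlay.
; The first overlap of the Collider by a ThirdPersonCharacter, gated by a DoOnce, plays each mesh's non-looping Vinestolight animation.
; A zero-length delay after playback starts precedes making them visible, so they appear already animating.
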(event OnComponentBeginOverlap(Collider)
  (params (OverlappedComponent :type Primitive%20Component%20Object%20Reference) (OtherActor :type Actor%20Object%20Reference) (OtherComp :type Primitive%20Component%20Object%20Reference) (OtherBodyIndex :type Integer) (bFromSweep :type Boolean) (SweepResult :type Hit%20Result%20Structure%20%28by%20ref%29))
  (Utilities|Casting|CastToThirdPersonCharacter OtherActor)
  (Utilities|FlowControl|DoOnce false
    (:Completed
      (Components|Animation|PlayAnimation (Variables|Default|GetSkeletalMeshComponent0) "/Game/GAME/Assets/City_Miscs/Growing_vines/Vinestolights/vinestolight_2.vinestolight_2_Animation" false)
      (Components|Animation|PlayAnimation (Variables|Default|GetSkeletalMeshComponent01) "/Game/GAME/Assets/City_Miscs/Growing_vines/Vinestolights/vinestolight.vinestolight_Animation" false)
      (Utilities|FlowControl|Delay 0.0)
      (Rendering|SetVisibility (Variables|Default|GetSkeletalMeshComponent01) true false)
      (Rendering|SetVisibility (Variables|Default|GetSkeletalMeshComponent0) true false))))

(event EventBeginPlay
  (Rendering|SetVisibility (Variables|Default|GetSkeletalMeshComponent01) false false)
  (Rendering|SetVisibility (Variables|Default|GetSkeletalMeshComponent0) false false))

(fn ConstructionScript
  (|CallParentFunction))