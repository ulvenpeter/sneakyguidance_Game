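; Park lightpole vine actor that plays a one-time growing animation when the player character reaches it.
; The skeletal mesh is hidden on BeginPlay, and its begin-overlap event casts to ThirdPersonCharacter before passing a DoOnce.
; It then starts the non-looping vine animation and makes the mesh visible after a zero-length delay.
; The Sequence repeats this identical logic in three branches on the same component.
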(event OnComponentBeginOverlap(SkeletalMeshComponent0)
  (params (OverlappedComponent :type Primitive%20Component%20Object%20Reference) (OtherActor :type Actor%20Object%20Reference) (OtherComp :type Primitive%20Component%20Object%20Reference) (OtherBodyIndex :type Integer) (bFromSweep :type Boolean) (SweepResult :type Hit%20Result%20Structure%20%28by%20ref%29))
  (Utilities|Casting|CastToThirdPersonCharacter OtherActor)
  (Utilities|FlowControl|DoOnce false
    (:Completed
      (Utilities|FlowControl|Sequence
        (:then_0
          (Components|Animation|PlayAnimation (Variables|Default|GetSkeletalMeshComponent0) "/Game/GAME/Assets/Park_vine_event/Lightpoles/SM_Lightpole_vine_1.SM_Lightpole_vine_1_Animation" false)
          (Utilities|FlowControl|Delay 0.0)
          (Rendering|SetVisibility (Variables|Default|GetSkeletalMeshComponent0) true false))
        (:then_1
          (Components|Animation|PlayAnimation (Variables|Default|GetSkeletalMeshComponent0) "/Game/GAME/Assets/Park_vine_event/Lightpoles/SM_Lightpole_vine_1.SM_Lightpole_vine_1_Animation" false)
          (Utilities|FlowControl|Delay 0.0)
          (Rendering|SetVisibility (Variables|Default|GetSkeletalMeshComponent0) true false))
        (:then_2
          (Components|Animation|PlayAnimation (Variables|Default|GetSkeletalMeshComponent0) "/Game/GAME/Assets/Park_vine_event/Lightpoles/SM_Lightpole_vine_1.SM_Lightpole_vine_1_Animation" false)
          (Utilities|FlowControl|Delay 0.0)
          (Rendering|SetVisibility (Variables|Default|GetSkeletalMeshComponent0) true false))))))

(event Collision|EventActorBeginOverlap
  (params (OtherActor :type Actor%20Object%20Reference))
  (|CallParentFunction OtherActor) ; This node is disabled and will not be called.\nDrag off pins to build functionality.
)

(event EventTick
  (params (DeltaSeconds :type Float%20%28single-precision%29))
  (|CallParentFunction DeltaSeconds) ; This node is disabled and will not be called.\nDrag off pins to build functionality.
)

(event EventBeginPlay
  (Rendering|SetVisibility (Variables|Default|GetSkeletalMeshComponent0) false false))

(fn ConstructionScript
  (|CallParentFunction))