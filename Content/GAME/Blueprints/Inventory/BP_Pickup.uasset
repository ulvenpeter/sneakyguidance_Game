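; Pickup actor for an equippable melee item that shows an equip prompt and damages what it hits.
; Entering the pickup overlap shows the player's EquipHud and sets CanEquip; leaving reverses both.
; Tick polls the player's EquippedToHand to set the mesh material and resize the pickup overlap from ScaleUp.
; A separate collider overlap applies test damage to non-player actors while the player's AttackingNormal is true.
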(event OnComponentBeginOverlap(Collider_Overlap)
  (params (OverlappedComponent :type Primitive%20Component%20Object%20Reference) (OtherActor :type Actor%20Object%20Reference) (OtherComp :type Primitive%20Component%20Object%20Reference) (OtherBodyIndex :type Integer) (bFromSweep :type Boolean) (SweepResult :type Hit%20Result%20Structure%20%28by%20ref%29))
  ;[1 1 1] Damage (test)
  (Utilities|Casting|CastToThirdPersonCharacter OtherActor
    (:CastFailed
      (bind _asthird_person_character (Utilities|Casting|CastToThirdPersonCharacter (Game|GetPlayerCharacter 0)))
      (if (Variables|/Game/GAME/New_Character/ThirdPersonCharacter.ThirdPersonCharacter_C|GetAttacking_Normal _asthird_person_character)
        (Game|Damage|ApplyDamage OtherActor 45.0 0 0 "/Script/Engine.DamageType")))))

(event OnComponentEndOverlap(Overlap_Pickup)
  (params (OverlappedComponent :type Primitive%20Component%20Object%20Reference) (OtherActor :type Actor%20Object%20Reference) (OtherComp :type Primitive%20Component%20Object%20Reference) (OtherBodyIndex :type Integer))
  (bind _asthird_person_character (Utilities|Casting|CastToThirdPersonCharacter OtherActor))
  (Widget|SetVisibility (Variables|/Game/GAME/New_Character/ThirdPersonCharacter.ThirdPersonCharacter_C|GetEquipHud _asthird_person_character) "Hidden")
  (Variables|Default|SetcanEquip false))

(event OnComponentBeginOverlap(Overlap_Pickup)
  (params (OverlappedComponent :type Primitive%20Component%20Object%20Reference) (OtherActor :type Actor%20Object%20Reference) (OtherComp :type Primitive%20Component%20Object%20Reference) (OtherBodyIndex :type Integer) (bFromSweep :type Boolean) (SweepResult :type Hit%20Result%20Structure%20%28by%20ref%29))
  (bind _asthird_person_character (Utilities|Casting|CastToThirdPersonCharacter OtherActor))
  (Utilities|FlowControl|Sequence
    (:then_0
      (Utilities|FlowControl|DoOnce false
        (:Completed
          (UserInterface|Viewport|AddtoViewport (Variables|/Game/GAME/New_Character/ThirdPersonCharacter.ThirdPersonCharacter_C|GetEquipHud _asthird_person_character) 0))))
    (:then_1
      (Widget|SetVisibility (Variables|/Game/GAME/New_Character/ThirdPersonCharacter.ThirdPersonCharacter_C|GetEquipHud _asthird_person_character) "Visible")
      (Variables|Default|SetcanEquip true))))

(event EventTick
  (params (DeltaSeconds :type Float%20%28single-precision%29))
  (bind _overlap_pickup (Variables|Default|GetOverlap_Pickup))
  ;[1 1 1] Destroy when picked up
  (bind _asthird_person_character (Utilities|Casting|CastToThirdPersonCharacter (Game|GetPlayerCharacter 0)))
  (if (Variables|/Game/GAME/New_Character/ThirdPersonCharacter.ThirdPersonCharacter_C|GetEquippedToHand _asthird_person_character)
    (Utilities|FlowControl|Sequence
      (:then_0
        (Utilities|FlowControl|DoOnce false :!label _label
          (:Completed
            (Rendering|Material|SetMaterial (Variables|Default|GetSkeletalMesh) 0 "/Game/GAME/Assets/City_Miscs/Pick_ups/Weapons/Baseball_bat/M_Wood_clean.M_Wood_clean")
            (goto _label Reset))))
      (:then_1
        (if (Variables|Default|GetScaleUp)
          (Transformation|SetRelativeScale3D _overlap_pickup "5.000000,5.000000,5.000000")
          (else
            (Transformation|SetRelativeScale3D _overlap_pickup "0.500000,0.500000,1.700000")))))))

(fn ConstructionScript)