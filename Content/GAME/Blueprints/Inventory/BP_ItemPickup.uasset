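; BP_ItemPickup is a world pickup that the player collects with E, with its mesh chosen by Index in the construction script.
; Overlap with ThirdPersonCharacter enables input and shows the character's AddPickupItem widget, added to the viewport once; leaving disables input and hides it.
; Pressing E adds KeyType to the character's OwnedKeys, destroys the actor, and passes Index to the first top-level BP_Inventory widget's AddItem.
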(event OnComponentBeginOverlap(Overlap)
  (params (OverlappedComponent :type Primitive%20Component%20Object%20Reference) (OtherActor :type Actor%20Object%20Reference) (OtherComp :type Primitive%20Component%20Object%20Reference) (OtherBodyIndex :type Integer) (bFromSweep :type Boolean) (SweepResult :type Hit%20Result%20Structure%20%28by%20ref%29))
  (bind _asthird_person_character (Utilities|Casting|CastToThirdPersonCharacter OtherActor))
  (Input|EnableInput (Game|GetPlayerController 0))
  (Utilities|FlowControl|Sequence
    (:then_0
      (Utilities|FlowControl|DoOnce false
        (:Completed
          (UserInterface|Viewport|AddtoViewport (Variables|/Game/GAME/New_Character/ThirdPersonCharacter.ThirdPersonCharacter_C|GetAdd_Pickup_Item _asthird_person_character) 0))))
    (:then_1
      (Widget|SetVisibility (Variables|/Game/GAME/New_Character/ThirdPersonCharacter.ThirdPersonCharacter_C|GetAdd_Pickup_Item _asthird_person_character) "Visible"))))

(event OnComponentEndOverlap(Overlap)
  (params (OverlappedComponent :type Primitive%20Component%20Object%20Reference) (OtherActor :type Actor%20Object%20Reference) (OtherComp :type Primitive%20Component%20Object%20Reference) (OtherBodyIndex :type Integer))
  (bind _asthird_person_character (Utilities|Casting|CastToThirdPersonCharacter OtherActor))
  (Input|DisableInput (Game|GetPlayerController 0))
  (Widget|SetVisibility (Variables|/Game/GAME/New_Character/ThirdPersonCharacter.ThirdPersonCharacter_C|GetAdd_Pickup_Item _asthird_person_character) "Hidden"))

(event Input|KeyboardEvents|E
  (params (Key :type Key%20Structure))
  (:Pressed
    (Utilities|FlowControl|Sequence
      (:then_0
        (Utilities|Array|Add (Variables|/Game/GAME/New_Character/ThirdPersonCharacter.ThirdPersonCharacter_C|GetOwnedKeys (stale OnComponentBeginOverlap(Overlap) _asthird_person_character)) (Variables|Default|GetKeyType))
        (Actor|DestroyActor))
      (:then_1
        (bind _foundwidgets (Widget|GetAllWidgetsOfClass "/Game/GAME/Blueprints/Inventory/BP_Inventory.BP_Inventory_C" true))
        (bind _asbp_inventory (Utilities|Casting|CastToBP_Inventory (Utilities|Array|Get(acopy) _foundwidgets)))
        (Default|AddItem _asbp_inventory (Variables|Default|GetIndex))))))

(fn ConstructionScript
  (Components|StaticMesh|SetStaticMesh (Variables|Default|GetStaticMesh) (Utilities|Array|Get(acopy) (Variables|Default|GetMeshes) (Variables|Default|GetIndex))))