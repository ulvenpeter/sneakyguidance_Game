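; BP_GasPickedUp is an interactable that lets the player flag gas in the inventory UI.
; Overlap of its Collider by a ThirdPersonCharacter enables input on the actor for player controller 0, and leaving disables it.
; While input is enabled, pressing E finds the first top-level BP_Inventory widget and sets its SetGasTexture flag to true.
; The actor is not destroyed or hidden here.
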(event OnComponentBeginOverlap(Collider)
  (params (OverlappedComponent :type Primitive%20Component%20Object%20Reference) (OtherActor :type Actor%20Object%20Reference) (OtherComp :type Primitive%20Component%20Object%20Reference) (OtherBodyIndex :type Integer) (bFromSweep :type Boolean) (SweepResult :type Hit%20Result%20Structure%20%28by%20ref%29))
  (Utilities|Casting|CastToThirdPersonCharacter OtherActor)
  (Input|EnableInput (Game|GetPlayerController 0)))

(event OnComponentEndOverlap(Collider)
  (params (OverlappedComponent :type Primitive%20Component%20Object%20Reference) (OtherActor :type Actor%20Object%20Reference) (OtherComp :type Primitive%20Component%20Object%20Reference) (OtherBodyIndex :type Integer))
  (Utilities|Casting|CastToThirdPersonCharacter OtherActor)
  (Input|DisableInput (Game|GetPlayerController 0)))

(event Input|KeyboardEvents|E
  (params (Key :type Key%20Structure))
  (:Pressed
    (bind _foundwidgets (Widget|GetAllWidgetsOfClass "/Game/GAME/Blueprints/Inventory/BP_Inventory.BP_Inventory_C" true))
    (bind _asbp_inventory (Utilities|Casting|CastToBP_Inventory (Utilities|Array|Get(acopy) _foundwidgets)))
    (Variables|/Game/GAME/Blueprints/Inventory/BP_Inventory.BP_Inventory_C|SetSetGasTexture _asbp_inventory true)))

(fn ConstructionScript)