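; Deer actor for the park that runs along a spline when the third-person character overlaps its trigger.
; After short delays, a timeline drives the mesh's swept transform along the spline and the run animation starts looping.
; Rotation is sampled in local space 180 units further along the spline than the location.
; A delay chained to the timeline update later switches to idle, then destroys the actor a second afterwards.
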(event OnComponentBeginOverlap(Trigger_deer)
  (params (OverlappedComponent :type Primitive%20Component%20Object%20Reference) (OtherActor :type Actor%20Object%20Reference) (OtherComp :type Primitive%20Component%20Object%20Reference) (OtherBodyIndex :type Integer) (bFromSweep :type Boolean) (SweepResult :type Hit%20Result%20Structure%20%28by%20ref%29))
  (bind _spline (Variables|Default|GetSpline))
  ;[1 1 1] Movement
  (Utilities|Casting|CastToThirdPersonCharacter OtherActor)
  (Utilities|FlowControl|Sequence
    (:then_0
      (Utilities|FlowControl|Delay 0.5)
      (bind _walkingpath (Timeline|Timeline_0 Play)
        (:Update
          (Transformation|SetWorldTransform (Variables|Default|GetDeer_02Run) (Math|Transform|MakeTransform (Spline|GetLocationatDistanceAlongSpline _spline (* _walkingpath (Spline|GetSplineLength _spline)) "World") (Spline|GetRotationatDistanceAlongSpline _spline (+ (* _walkingpath (Spline|GetSplineLength _spline)) 1.8e+02) "Local")) true false)
          (Utilities|FlowControl|Delay 18.0)
          (Components|Animation|PlayAnimation (Variables|Default|GetDeer_02Run) "/Game/GAME/Assets/Deer/Deer_01Idle_Anim.Deer_01Idle_Anim" true)
          (Utilities|FlowControl|Delay 1.0)
          (Actor|DestroyActor))))
    (:then_1
      (Utilities|FlowControl|Delay 2.8)
      (Components|Animation|PlayAnimation (Variables|Default|GetDeer_02Run) "/Game/GAME/Assets/Deer/Deer_02Run_Anim.Deer_02Run_Anim" true))))

(fn ConstructionScript)