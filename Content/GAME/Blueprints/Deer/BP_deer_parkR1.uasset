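; BP_deer_parkR1 is a deer actor that moves along a spline path.
; Tick, via a short delay, plays a timeline whose Walkingpath track positions and rotates Deer02Run along the spline with sweep.
; A parallel Tick branch uses delays to alternate the animation Blueprint's Speed between fast and slow values.
; The Trigger_deer overlap only casts to ThirdPersonCharacter and drives nothing.
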(event OnComponentBeginOverlap(Trigger_deer)
  (params (OverlappedComponent :type Primitive%20Component%20Object%20Reference) (OtherActor :type Actor%20Object%20Reference) (OtherComp :type Primitive%20Component%20Object%20Reference) (OtherBodyIndex :type Integer) (bFromSweep :type Boolean) (SweepResult :type Hit%20Result%20Structure%20%28by%20ref%29))
  (Utilities|Casting|CastToThirdPersonCharacter OtherActor))

(event EventTick
  (params (DeltaSeconds :type Float%20%28single-precision%29))
  (bind _spline (Variables|Default|GetSpline))
  (Utilities|FlowControl|Sequence
    (:then_0
      (Utilities|FlowControl|Delay 0.5)
      (bind _walkingpath (Timeline|Timeline_0 Play)
        (:Update
          (Transformation|SetWorldTransform (Variables|Default|GetDeer_02Run) (Math|Transform|MakeTransform (Spline|GetLocationatDistanceAlongSpline _spline (* _walkingpath (Spline|GetSplineLength _spline)) "World") (Spline|GetRotationatDistanceAlongSpline _spline (* _walkingpath (Spline|GetSplineLength _spline)) "Local")) true false))))
    (:then_1
      (Utilities|FlowControl|Delay 0.5)
      (Variables|/Game/GAME/Assets/Deer/Deer_Animbp.Deer_Animbp_C|SetSpeed (Variables|Default|GetDeer%20Animbp) 75.0)
      (Utilities|FlowControl|Delay 3.0)
      (Variables|/Game/GAME/Assets/Deer/Deer_Animbp.Deer_Animbp_C|SetSpeed (Variables|Default|GetDeer%20Animbp) 23.0))))

(fn ConstructionScript)