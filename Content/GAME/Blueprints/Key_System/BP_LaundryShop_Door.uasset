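; Laundry shop door that the player swings open or shut with E while inside its overlap volume.
; Overlap toggles input and prints an on-screen prompt; E plays or reverses a rotation timeline based on IsClosed, which is re-evaluated from the angle when the swing finishes.
; Timeline updates also trigger squeak and shop chime sound events through chained DoOnce gates, with only the squeak gate reset after each swing.
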(event OnComponentBeginOverlap(Overlap)
  (params (OverlappedComponent :type Primitive%20Component%20Object%20Reference) (OtherActor :type Actor%20Object%20Reference) (OtherComp :type Primitive%20Component%20Object%20Reference) (OtherBodyIndex :type Integer) (bFromSweep :type Boolean) (SweepResult :type Hit%20Result%20Structure%20%28by%20ref%29))
  (Utilities|Casting|CastToThirdPersonCharacter OtherActor)
  (Input|EnableInput (Game|GetPlayerController 0))
  (Development|PrintString "PRESS E TO OPEN" true true "(R=0.012200,G=1.000000,B=0.000000,A=1.000000)" 3.0))

(event OnComponentEndOverlap(Overlap)
  (params (OverlappedComponent :type Primitive%20Component%20Object%20Reference) (OtherActor :type Actor%20Object%20Reference) (OtherComp :type Primitive%20Component%20Object%20Reference) (OtherBodyIndex :type Integer))
  (Utilities|Casting|CastToThirdPersonCharacter OtherActor)
  (Input|DisableInput (Game|GetPlayerController 0)))

(event Input|KeyboardEvents|E
  (params (Key :type Key%20Structure))
  (bind _returnvalue (Transformation|GetActorLocation))
  (:Pressed
    (if (Variables|Default|GetIsClosed)
      (bind _doorrot (Timeline|DoorRotation Play)
        (:Update
          (Utilities|FlowControl|Sequence
            (:then_0
              (Transformation|SetRelativeRotation (Variables|Default|GetStaticMesh) (Math|Rotator|MakeRotator 0.0 0.0 _doorrot) false false))
            (:then_1
              (Utilities|FlowControl|DoOnce true :!label _label
                (:Completed
                  (Class|FMODBlueprintStatics|PlayEventatLocation "/Game/FMOD/Events/Buildings/DoorSqueaky.DoorSqueaky" (Math|Conversions|ToTransform(Vector) _returnvalue))
                  (Utilities|FlowControl|DoOnce false
                    (:Completed
                      (Class|FMODBlueprintStatics|PlayEventatLocation "/Game/FMOD/Events/Buildings/ShopPLing.ShopPLing" (Math|Conversions|ToTransform(Vector) _returnvalue)))))))))
        (:Finished
          (Utilities|FlowControl|Sequence
            (:then_0
              (goto _label Reset))
            (:then_1
              (Variables|Default|SetIsClosed (< _doorrot 91.0))))))
      (else
        (Timeline|DoorRotation Reverse)))))

(fn ConstructionScript)