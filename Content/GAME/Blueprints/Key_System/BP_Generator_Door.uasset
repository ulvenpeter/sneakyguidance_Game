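; BP_Generator_Door is a double door the player opens by pressing E while near it.
; Two overlap volumes toggle input for the ThirdPersonCharacter, and the second also prints an on-screen prompt.
; E plays two timelines that yaw the door meshes, with a DoOnce firing a metal door sound event at the actor's location.
; The graph has no key check or closing logic.
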(event OnComponentBeginOverlap(Overlap1)
  (params (OverlappedComponent :type Primitive%20Component%20Object%20Reference) (OtherActor :type Actor%20Object%20Reference) (OtherComp :type Primitive%20Component%20Object%20Reference) (OtherBodyIndex :type Integer) (bFromSweep :type Boolean) (SweepResult :type Hit%20Result%20Structure%20%28by%20ref%29))
  (Utilities|Casting|CastToThirdPersonCharacter OtherActor)
  (Input|EnableInput (Game|GetPlayerController 0))
  (Development|PrintString "PRESS E TO OPEN" true true "(R=0.012200,G=1.000000,B=0.000000,A=1.000000)" 3.0))

(event OnComponentEndOverlap(Overlap1)
  (params (OverlappedComponent :type Primitive%20Component%20Object%20Reference) (OtherActor :type Actor%20Object%20Reference) (OtherComp :type Primitive%20Component%20Object%20Reference) (OtherBodyIndex :type Integer))
  (Utilities|Casting|CastToThirdPersonCharacter OtherActor)
  (Input|DisableInput (Game|GetPlayerController 0)))

(event OnComponentBeginOverlap(Overlap)
  (params (OverlappedComponent :type Primitive%20Component%20Object%20Reference) (OtherActor :type Actor%20Object%20Reference) (OtherComp :type Primitive%20Component%20Object%20Reference) (OtherBodyIndex :type Integer) (bFromSweep :type Boolean) (SweepResult :type Hit%20Result%20Structure%20%28by%20ref%29))
  (Utilities|Casting|CastToThirdPersonCharacter OtherActor)
  (Input|EnableInput (Game|GetPlayerController 0)))

(event OnComponentEndOverlap(Overlap)
  (params (OverlappedComponent :type Primitive%20Component%20Object%20Reference) (OtherActor :type Actor%20Object%20Reference) (OtherComp :type Primitive%20Component%20Object%20Reference) (OtherBodyIndex :type Integer))
  (Utilities|Casting|CastToThirdPersonCharacter OtherActor)
  (Input|DisableInput (Game|GetPlayerController 0)))

(event Input|KeyboardEvents|E
  (params (Key :type Key%20Structure))
  (:Pressed
    (Utilities|FlowControl|Sequence
      (:then_0
        (bind _gendoor1 (Timeline|Gen_door1 Play)
          (:Update
            (Transformation|SetRelativeRotation (Variables|Default|GetStaticMesh) (Math|Rotator|MakeRotator 0.0 0.0 _gendoor1) false false))))
      (:then_1
        (bind _gendoor2 (Timeline|Gen_door_2 Play)
          (:Update
            (Transformation|SetRelativeRotation (Variables|Default|GetStaticMesh1) (Math|Rotator|MakeRotator 0.0 0.0 _gendoor2) false false)
            (Utilities|FlowControl|DoOnce false
              (:Completed
                (Class|FMODBlueprintStatics|PlayEventatLocation "/Game/FMOD/Events/Buildings/MetalDoor.MetalDoor" (Math|Conversions|ToTransform(Vector) (Transformation|GetActorLocation)))))))))))

(fn ConstructionScript)