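; Generator start actor in the key system that starts the generator once a cogwheel (BP_TannHjul) is enabled and gasoline (BP_Gasolina) is added.
; Every Tick it gathers both actor classes through empty loops, so the check reads only each loop's last element.
; When both flags are true, a DoOnce plays the Generator sound event at the actor's location and sets GeneratorStarted.
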(event EventTick
  (params (DeltaSeconds :type Float%20%28single-precision%29))
  (Utilities|FlowControl|Sequence
    (:then_0
      (bind _outactors (Actor|GetAllActorsOfClass "/Game/GAME/Blueprints/Key_System/BP_TannHjul.BP_TannHjul_C"))
      (bind _array_element (Utilities|Array|ForEachLoopwithBreak _outactors)))
    (:then_1
      (bind _outactors_2 (Actor|GetAllActorsOfClass "/Game/GAME/Blueprints/Key_System/BP_Gasolina.BP_Gasolina_C"))
      (bind _array_element_2 (Utilities|Array|ForEachLoopwithBreak _outactors_2)))
    (:then_2
      (if (and (Variables|/Game/GAME/Blueprints/Key_System/BP_TannHjul.BP_TannHjul_C|GetTannHjul_enabled _array_element) (Variables|/Game/GAME/Blueprints/Key_System/BP_Gasolina.BP_Gasolina_C|GetGas_Added _array_element_2))
        (Utilities|FlowControl|DoOnce false
          (:Completed
            (Class|FMODBlueprintStatics|PlayEventatLocation "/Game/FMOD/Events/Buildings/Generator.Generator" (Math|Conversions|ToTransform(Vector) (Transformation|GetActorLocation)))
            (Variables|Default|SetGeneratorStarted true)))))))

(fn ConstructionScript)