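; BP_ElevatorDoor2 is a sliding elevator door that opens for the ThirdPersonCharacter once generator power is on.
; On overlap it loops over all BP_GeneratorStart actors with an empty body, then checks GeneratorStarted on the last element.
; If powered, a timeline offsets the door from its BeginPlay position; otherwise it prints a no-power message.
; Leaving the overlap reverses the timeline after a short delay.
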(event OnComponentBeginOverlap(Overlap)
  (params (OverlappedComponent :type Primitive%20Component%20Object%20Reference) (OtherActor :type Actor%20Object%20Reference) (OtherComp :type Primitive%20Component%20Object%20Reference) (OtherBodyIndex :type Integer) (bFromSweep :type Boolean) (SweepResult :type Hit%20Result%20Structure%20%28by%20ref%29))
  (Utilities|Casting|CastToThirdPersonCharacter OtherActor)
  (Utilities|FlowControl|Sequence
    (:then_0
      (bind _outactors (Actor|GetAllActorsOfClass "/Game/GAME/Blueprints/Key_System/BP_GeneratorStart.BP_GeneratorStart_C"))
      (bind _array_element (Utilities|Array|ForEachLoopwithBreak _outactors)))
    (:then_1
      (if (Variables|/Game/GAME/Blueprints/Key_System/BP_GeneratorStart.BP_GeneratorStart_C|GetGeneratorStarted _array_element)
        (bind _slidingdoor (Timeline|Timeline_0 Play)
          (:Update
            (Transformation|SetActorLocation (+ _slidingdoor (Variables|Default|GetStartingPosition)) false false)))
        (else
          (Development|PrintString "Seems like i need power.." true true "(R=1.000000,G=0.080133,B=0.000000,A=1.000000)"))))))

(event OnComponentEndOverlap(Overlap)
  (params (OverlappedComponent :type Primitive%20Component%20Object%20Reference) (OtherActor :type Actor%20Object%20Reference) (OtherComp :type Primitive%20Component%20Object%20Reference) (OtherBodyIndex :type Integer))
  (Utilities|Casting|CastToThirdPersonCharacter OtherActor)
  (Utilities|FlowControl|Delay 1.0)
  (bind _slidingdoor (Timeline|Timeline_0 Reverse)
    (:Update
      (Transformation|SetActorLocation (+ _slidingdoor (Variables|Default|GetStartingPosition)) false false))))

(event EventBeginPlay
  (Variables|Default|SetStartingPosition (Transformation|GetActorLocation)))

(fn ConstructionScript)