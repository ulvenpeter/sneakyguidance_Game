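; Key-locked actor, apparently a door, that swings open when a ThirdPersonCharacter carrying the matching key enters one of its two trigger volumes.
; Each overlap searches the character's OwnedKeys for RequireKeyType, removes a match and rotates the whole actor a quarter turn, in opposite directions per trigger.
; The loop has no break, and the code copying keys to BP_TestGameInstance is never run.
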(event OnComponentBeginOverlap(Overlap)
  (params (OverlappedComponent :type Primitive%20Component%20Object%20Reference) (OtherActor :type Actor%20Object%20Reference) (OtherComp :type Primitive%20Component%20Object%20Reference) (OtherBodyIndex :type Integer) (bFromSweep :type Boolean) (SweepResult :type Hit%20Result%20Structure%20%28by%20ref%29))
  (bind _asthird_person_character (Utilities|Casting|CastToThirdPersonCharacter OtherActor))
  (for (_array_element _array_index) (Variables|/Game/GAME/New_Character/ThirdPersonCharacter.ThirdPersonCharacter_C|GetOwnedKeys _asthird_person_character)
    (if (Utilities|Enum|Equal(Enum) _array_element (Variables|Default|GetRequire%20Key%20Type))
      (Utilities|Array|RemoveIndex (Variables|/Game/GAME/New_Character/ThirdPersonCharacter.ThirdPersonCharacter_C|GetOwnedKeys _asthird_person_character) _array_index)
      (Development|PrintString "")
      (Transformation|AddActorLocalRotation "0,90.000000, 0" true false))))

(event OnComponentBeginOverlap(Overlap1)
  (params (OverlappedComponent :type Primitive%20Component%20Object%20Reference) (OtherActor :type Actor%20Object%20Reference) (OtherComp :type Primitive%20Component%20Object%20Reference) (OtherBodyIndex :type Integer) (bFromSweep :type Boolean) (SweepResult :type Hit%20Result%20Structure%20%28by%20ref%29))
  (bind _asthird_person_character (Utilities|Casting|CastToThirdPersonCharacter OtherActor))
  (for (_array_element _array_index) (Variables|/Game/GAME/New_Character/ThirdPersonCharacter.ThirdPersonCharacter_C|GetOwnedKeys _asthird_person_character)
    (if (Utilities|Enum|Equal(Enum) _array_element (Variables|Default|GetRequire%20Key%20Type))
      (Utilities|Array|RemoveIndex (Variables|/Game/GAME/New_Character/ThirdPersonCharacter.ThirdPersonCharacter_C|GetOwnedKeys _asthird_person_character) _array_index)
      (Development|PrintString "")
      (Transformation|AddActorLocalRotation "0,-90.000000, 0" true false))))

(fn ConstructionScript)