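; BP_Gasolina is a Key System interactable where the player uses a required key item to add gasolina (gas).
; Overlapping enables E input and shows the character's AddGas prompt until gas is added; leaving hides it.
; E scans OwnedKeys, removes the RequireKeyType match, copies keys to TestGameInstance, plays the Gasoline sound event, and sets GasAdded after a delay.
; "Need Gas" prints for each non-matching key, so an empty inventory prints nothing.
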(event OnComponentBeginOverlap(Overlap)
  (params (OverlappedComponent :type Primitive%20Component%20Object%20Reference) (OtherActor :type Actor%20Object%20Reference) (OtherComp :type Primitive%20Component%20Object%20Reference) (OtherBodyIndex :type Integer) (bFromSweep :type Boolean) (SweepResult :type Hit%20Result%20Structure%20%28by%20ref%29))
  (bind _asthird_person_character (Utilities|Casting|CastToThirdPersonCharacter OtherActor))
  (Input|EnableInput (Game|GetPlayerController 0))
  (if (not (Variables|Default|GetGas_Added))
    (Utilities|FlowControl|Sequence
      (:then_0
        (Utilities|FlowControl|DoOnce false
          (:Completed
            (UserInterface|Viewport|AddtoViewport (Variables|/Game/GAME/New_Character/ThirdPersonCharacter.ThirdPersonCharacter_C|GetAdd_Gas _asthird_person_character) 0))))
      (:then_1
        (Widget|SetVisibility (Variables|/Game/GAME/New_Character/ThirdPersonCharacter.ThirdPersonCharacter_C|GetAdd_Gas _asthird_person_character) "Visible")))))

(event OnComponentEndOverlap(Overlap)
  (params (OverlappedComponent :type Primitive%20Component%20Object%20Reference) (OtherActor :type Actor%20Object%20Reference) (OtherComp :type Primitive%20Component%20Object%20Reference) (OtherBodyIndex :type Integer))
  (bind _asthird_person_character (Utilities|Casting|CastToThirdPersonCharacter OtherActor))
  (Input|DisableInput (Game|GetPlayerController 0))
  (Widget|SetVisibility (Variables|/Game/GAME/New_Character/ThirdPersonCharacter.ThirdPersonCharacter_C|GetAdd_Gas _asthird_person_character) "Hidden"))

(event Input|KeyboardEvents|E
  (params (Key :type Key%20Structure))
  (:Pressed
    (for (_array_element _array_index) (Variables|/Game/GAME/New_Character/ThirdPersonCharacter.ThirdPersonCharacter_C|GetOwnedKeys (stale OnComponentBeginOverlap(Overlap) _asthird_person_character))
      (if (Utilities|Enum|Equal(Enum) _array_element (Variables|Default|GetRequire%20Key%20Type))
        (Utilities|Array|RemoveIndex (Variables|/Game/GAME/New_Character/ThirdPersonCharacter.ThirdPersonCharacter_C|GetOwnedKeys (stale OnComponentBeginOverlap(Overlap) _asthird_person_character)) _array_index)
        (bind _astest_game_instance (Utilities|Casting|CastToTestGameInstance (Game|GetGameInstance)))
        (Variables|/Game/GAME/Blueprints/Key_System/TestGameInstance.TestGameInstance_C|SetPlayerKeys _astest_game_instance (Variables|/Game/GAME/New_Character/ThirdPersonCharacter.ThirdPersonCharacter_C|GetOwnedKeys (stale OnComponentBeginOverlap(Overlap) _asthird_person_character)))
        (Class|FMODBlueprintStatics|PlayEventatLocation "/Game/FMOD/Events/Buildings/Gasoline.Gasoline" (Math|Conversions|ToTransform(Vector) (Transformation|GetActorLocation)))
        (Widget|SetVisibility (Variables|/Game/GAME/New_Character/ThirdPersonCharacter.ThirdPersonCharacter_C|GetAdd_Gas (stale OnComponentBeginOverlap(Overlap) _asthird_person_character)) "Hidden")
        (Utilities|FlowControl|Delay 1.3)
        (if true
          (Variables|Default|SetGas_Added true))
        (else
          (Development|PrintString "Need Gas" true true "(R=1.000000,G=0.000000,B=0.016751,A=1.000000)" 3.0))))))

(fn ConstructionScript)