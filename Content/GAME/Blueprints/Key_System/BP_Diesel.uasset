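; BP_Diesel is a pickup actor in the key system that adds its KeyType to the third-person character's OwnedKeys.
; Overlapping the character enables input and shows its PickupGas prompt, added to the viewport once; leaving disables input and hides it.
; Pressing E records the key on the character and destroys the actor.
; The construction script chooses the mesh material from KeyType, with none assigned for Diesel or ElectricWire.
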(event OnComponentBeginOverlap(Overlap)
  (params (OverlappedComponent :type Primitive%20Component%20Object%20Reference) (OtherActor :type Actor%20Object%20Reference) (OtherComp :type Primitive%20Component%20Object%20Reference) (OtherBodyIndex :type Integer) (bFromSweep :type Boolean) (SweepResult :type Hit%20Result%20Structure%20%28by%20ref%29))
  (bind _asthird_person_character (Utilities|Casting|CastToThirdPersonCharacter OtherActor))
  (Input|EnableInput (Game|GetPlayerController 0))
  (Utilities|FlowControl|Sequence
    (:then_0
      (Utilities|FlowControl|DoOnce false
        (:Completed
          (UserInterface|Viewport|AddtoViewport (Variables|/Game/GAME/New_Character/ThirdPersonCharacter.ThirdPersonCharacter_C|GetPickup_Gas _asthird_person_character) 0))))
    (:then_1
      (Widget|SetVisibility (Variables|/Game/GAME/New_Character/ThirdPersonCharacter.ThirdPersonCharacter_C|GetPickup_Gas _asthird_person_character) "Visible"))))

(event OnComponentEndOverlap(Overlap)
  (params (OverlappedComponent :type Primitive%20Component%20Object%20Reference) (OtherActor :type Actor%20Object%20Reference) (OtherComp :type Primitive%20Component%20Object%20Reference) (OtherBodyIndex :type Integer))
  (bind _asthird_person_character (Utilities|Casting|CastToThirdPersonCharacter OtherActor))
  (Input|DisableInput (Game|GetPlayerController 0))
  (Widget|SetVisibility (Variables|/Game/GAME/New_Character/ThirdPersonCharacter.ThirdPersonCharacter_C|GetPickup_Gas _asthird_person_character) "Hidden"))

(event Input|KeyboardEvents|E
  (params (Key :type Key%20Structure))
  (:Pressed
    (Utilities|Array|Add (Variables|/Game/GAME/New_Character/ThirdPersonCharacter.ThirdPersonCharacter_C|GetOwnedKeys (stale OnComponentBeginOverlap(Overlap) _asthird_person_character)) (Variables|Default|GetKeyType))
    (Actor|DestroyActor)))

(fn ConstructionScript
  (Rendering|Material|SetMaterial (Variables|Default|GetStaticMesh) 0 (Utilities|Select :Index (Variables|Default|GetKeyType) :NewEnumerator0 "/Game/GAME/Blueprints/Key_System/M_Key.M_Key" :NewEnumerator1 "/Game/GAME/Blueprints/Key_System/M_BlueKey.M_BlueKey" :NewEnumerator2 "/Game/GAME/Blueprints/Key_System/M_RedKey.M_RedKey" :NewEnumerator3 "/Game/GAME/Blueprints/Key_System/M_GreenKey.M_GreenKey" :NewEnumerator4 "/Game/GAME/Assets/Buildings/laundryshop/belt/M_02_-_Default.M_02_-_Default" :NewEnumerator5 0 :NewEnumerator6 0)))