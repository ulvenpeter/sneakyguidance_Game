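; BP_Skytower_Lobby_Door1 is a sliding lobby door that opens when a ThirdPersonCharacter enters its overlap volume.
; A timeline offsets the whole actor from the location saved at BeginPlay, then reverses one second after the character leaves.
; A DoOnce plays the Lightbuzzing sound event once per movement and resets when the timeline finishes.
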(event OnComponentBeginOverlap(Overlap)
  (params (OverlappedComponent :type Primitive%20Component%20Object%20Reference) (OtherActor :type Actor%20Object%20Reference) (OtherComp :type Primitive%20Component%20Object%20Reference) (OtherBodyIndex :type Integer) (bFromSweep :type Boolean) (SweepResult :type Hit%20Result%20Structure%20%28by%20ref%29))
  (Utilities|Casting|CastToThirdPersonCharacter OtherActor)
  (bind _slidingdoor (Timeline|SlidingDoor1 Play)
    (:Update
      (Utilities|FlowControl|Sequence
        (:then_0
          (Utilities|FlowControl|DoOnce false :!label _label
            (:Completed
              (Class|FMODBlueprintStatics|PlayEventatLocation "/Game/FMOD/Events/Buildings/Lightbuzzing.Lightbuzzing" (Math|Conversions|ToTransform(Vector) (Transformation|GetActorLocation))))))
        (:then_1
          (Transformation|SetActorLocation (+ _slidingdoor (Variables|Default|GetStartingPosition)) false false))))
    (:Finished
      (goto _label Reset))))

(event OnComponentEndOverlap(Overlap)
  (params (OverlappedComponent :type Primitive%20Component%20Object%20Reference) (OtherActor :type Actor%20Object%20Reference) (OtherComp :type Primitive%20Component%20Object%20Reference) (OtherBodyIndex :type Integer))
  (Utilities|Casting|CastToThirdPersonCharacter OtherActor)
  (Utilities|FlowControl|Delay 1.0)
  (bind _slidingdoor (Timeline|SlidingDoor1 Reverse)
    (:Update
      (Utilities|FlowControl|Sequence
        (:then_0
          (Utilities|FlowControl|DoOnce false :!label _label
            (:Completed
              (Class|FMODBlueprintStatics|PlayEventatLocation "/Game/FMOD/Events/Buildings/Lightbuzzing.Lightbuzzing" (Math|Conversions|ToTransform(Vector) (Transformation|GetActorLocation))))))
        (:then_1
          (Transformation|SetActorLocation (+ _slidingdoor (Variables|Default|GetStartingPosition)) false false))))
    (:Finished
      (goto _label Reset))))

(event EventBeginPlay
  (Variables|Default|SetStartingPosition (Transformation|GetActorLocation)))

(fn ConstructionScript)