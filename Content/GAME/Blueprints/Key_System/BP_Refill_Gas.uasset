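; BP_Refill_Gas is an interactable gas pickup in the key system, granting the player its KeyType.
; Overlap by the ThirdPersonCharacter enables input and shows the character's PickupGas widget, while leaving disables input and hides it.
; Pressing E adds KeyType to the character's OwnedKeys and destroys the overlap component.
; It also plays the Gasoline sound event once and swaps two gas meshes to non-glowing materials.
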(event OnComponentBeginOverlap(Overlap)
  (params (OverlappedComponent :type Primitive%20Component%20Object%20Reference) (OtherActor :type Actor%20Object%20Reference) (OtherComp :type Primitive%20Component%20Object%20Reference) (OtherBodyIndex :type Integer) (bFromSweep :type Boolean) (SweepResult :type Hit%20Result%20Structure%20%28by%20ref%29))
  (bind _asthird_person_character (Utilities|Casting|CastToThirdPersonCharacter OtherActor))
  (Input|EnableInput (Game|GetPlayerController 0))
  (Utilities|FlowControl|Sequence
    (:then_0
      (Utilities|FlowControl|DoOnce false
        (:Completed
          (UserInterface|Viewport|AddtoViewport (Variables|/Game/GAME/New_Character/ThirdPersonCharacter.ThirdPersonCharacter_C|GetPickup_Gas _asthird_person_character) 0))))
    (:then_1
      (Widget|SetVisibility (Variables|/Game/GAME/New_Character/ThirdPersonCharacter.ThirdPersonCharacter_C|GetPickup_Gas _asthird_person_character) "Visible"))))

(event OnComponentEndOverlap(Overlap)
  (params (OverlappedComponent :type Primitive%20Component%20Object%20Reference) (OtherActor :type Actor%20Object%20Reference) (OtherComp :type Primitive%20Component%20Object%20Reference) (OtherBodyIndex :type Integer))
  (bind _asthird_person_character (Utilities|Casting|CastToThirdPersonCharacter OtherActor))
  (Input|DisableInput (Game|GetPlayerController 0))
  (Widget|SetVisibility (Variables|/Game/GAME/New_Character/ThirdPersonCharacter.ThirdPersonCharacter_C|GetPickup_Gas _asthird_person_character) "Hidden"))

(event Input|KeyboardEvents|E
  (params (Key :type Key%20Structure))
  (bind _sm_gas2 (Variables|Default|GetSM_gas2))
  (:Pressed
    (Utilities|FlowControl|Sequence
      (:then_0
        (Utilities|Array|Add (Variables|/Game/GAME/New_Character/ThirdPersonCharacter.ThirdPersonCharacter_C|GetOwnedKeys (stale OnComponentBeginOverlap(Overlap) _asthird_person_character)) (Variables|Default|GetKeyType))
        (Components|DestroyComponent (Variables|Default|GetOverlap)))
      (:then_1
        (Utilities|FlowControl|DoOnce false
          (:Completed
            (Class|FMODBlueprintStatics|PlayEventatLocation "/Game/FMOD/Events/Buildings/Gasoline.Gasoline" (Math|Conversions|ToTransform(Vector) (Transformation|GetActorLocation)))
            (Utilities|FlowControl|Sequence
              (:then_0
                (Rendering|Material|SetMaterial _sm_gas2 12 "/Game/GAME/Assets/Gass_Station/M_steel_noglow.M_steel_noglow"))
              (:then_1
                (Rendering|Material|SetMaterial _sm_gas2 13 "/Game/GAME/Assets/Gass_Station/M_Green_noglow.M_Green_noglow")))))))))

(fn ConstructionScript)