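; BP_Projectile is a homing projectile actor in the zombie-killing VFX folder that damages its target and bursts on contact.
; HomingLight adds a static mesh component to a valid target as the homing point, enables high-acceleration homing and applies damage immediately, without waiting for impact.
; After a short delay it destroys the Projectile and Sphere components.
; The first collision hit fires a radial impulse, spawns a particle emitter and destroys the actor.
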(event OnComponentHit(Collision)
  (params (HitComponent :type Primitive%20Component%20Object%20Reference) (OtherActor :type Actor%20Object%20Reference) (OtherComp :type Primitive%20Component%20Object%20Reference) (NormalImpulse :type Vector :default "0, 0, 0") (Hit :type Hit%20Result%20Structure%20%28by%20ref%29))
  (bind _hitforce (Variables|Default|GetHitForce))
  ;[1 1 1] VFx On Contact
  (Utilities|FlowControl|DoOnce false
    (:Completed
      (Class|RadialForceComponent|FireImpulse _hitforce)
      (Effects|SpawnEmitteratLocation 0 (Transformation|GetWorldLocation _hitforce))
      (Actor|DestroyActor))))

(event Custom|HomingLight
  (params (TargetToHit :type CH%20Zombie%20Police%20Object%20Reference))
  (bind _projectile (Variables|Default|GetProjectile))
  (if (Utilities|IsValid TargetToHit)
    (bind _returnvalue (AddComponent|AddStaticMeshComponent TargetToHit false))
    (Variables|/Script/Engine.ProjectileMovementComponent|SetHomingTargetComponent _projectile _returnvalue)
    (Variables|/Script/Engine.ProjectileMovementComponent|SetbIsHomingProjectile _projectile true)
    (Variables|/Script/Engine.ProjectileMovementComponent|SetHomingAccelerationMagnitude _projectile 1e+05)
    (Default|HealthInterfaceDamage TargetToHit 1e+02)
    (Utilities|FlowControl|Delay 1.0)
    (Components|DestroyComponent (Variables|Default|GetProjectile))))

(fn ConstructionScript)