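; Zombie enemy Blueprint that roams the navmesh, chases the player on sight and shows a floating health bar.
; Tick updates the bar, yaws it toward the player, destroys the zombie at zero health and starts random roam moves while Inrange is false.
; PawnSensing sets Inrange and moves to the seen player character, clearing the flag only after a successful move and short delay.
; A line trace node is left unconnected.
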(event OnSeePawn(PawnSensing)
  (params (Pawn :type Pawn%20Object%20Reference))
  ;[0 0.5876 1] Roaming
  (Variables|Default|SetInrange true)
  (bind _asbp_third_person_character (Utilities|Casting|CastToBP_ThirdPersonCharacter Pawn))
  (AI|AIMoveTo self "0, 0, 0" _asbp_third_person_character 5.0 false
    (:then
      (Variables|Default|SetInrange true))
    (:OnSuccess
      (Utilities|FlowControl|Delay 3.0)
      (Variables|Default|SetInrange false))))

(event EventTick
  (params (DeltaSeconds :type Float%20%28single-precision%29))
  (bind _widget (Variables|Default|GetWidget))
  ;[0.4323 0.01168 0] AI Health
  (Utilities|FlowControl|Sequence
    (:then_0
      (bind _asbp_ai_health (Utilities|Casting|CastToBP_AI_Health (UserInterface|GetUserWidgetObject (Variables|Default|GetWidget))))
      (Progress|SetPercent (Variables|/Game/GAME/Character/Zombie/BP_AI_Health.BP_AI_Health_C|GetProgressBar_140 _asbp_ai_health) (/ (Variables|Default|GetAI_Health) 1e+02))
      (Transformation|SetWorldRotation _widget (Math|Rotator|MakeRotator 0.0 0.0 (.Yaw (Math|Rotator|BreakRotator (Math|Rotator|FindLookatRotation (Transformation|GetWorldLocation _widget) (Transformation|GetActorLocation (Game|GetPlayerCharacter 0)))))) false false)
      (if (<= (Variables|Default|GetAI_Health) 0.0)
        (Actor|DestroyActor)))
    (:then_1
      ;[0 0.5876 1] Roaming
      (if (not (Variables|Default|GetInrange))
        (if (not (Variables|Default|GetMoving))
          (AI|AIMoveTo self (.RandomLocation (Class|NavigationSystem|GetRandomPointinNavigableRadius (Transformation|GetActorLocation) 5e+03)) 0 5.0 false
            (:then
              (Variables|Default|SetMoving true))
            (:OnSuccess
              (Variables|Default|SetMoving false :!label _label))
            (:OnFail
              (goto _label))))))))

(fn ConstructionScript)