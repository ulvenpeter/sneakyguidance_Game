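; BP_CryopodLight is a point light, named for a cryopod, that blinks on and off at a steady interval.
; BeginPlay hides the light, then sets a start flag after a short delay.
; Once flagged, Tick drives a DoOnce gate that waits on a fixed delay, toggles visibility, then resets itself to repeat.
; A random-float calculation is present but unused, so the blink timing does not vary.
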(event EventTick
  (params (DeltaSeconds :type Float%20%28single-precision%29))
  (if (Variables|Default|GetStartLight)
    (Utilities|FlowControl|DoOnce false :!label _label
      (:Completed
        (Utilities|FlowControl|RetriggerableDelay 1.45)
        (Rendering|ToggleVisibility (Variables|Default|GetPointLight) false)
        (goto _label Reset)))))

(event EventBeginPlay
  (Rendering|SetVisibility (Variables|Default|GetPointLight) false false)
  (Utilities|FlowControl|Delay 1.5)
  (Variables|Default|SetStartLight true))

(fn ConstructionScript)