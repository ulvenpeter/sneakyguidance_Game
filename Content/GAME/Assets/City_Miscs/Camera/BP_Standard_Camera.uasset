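; A city prop camera actor that turns to face the player character and blinks a point light.
; Each tick it computes a look-at rotation from the camera mesh to player 0, applies fixed pitch and yaw offsets, and zeroes roll.
; A DoOnce gate around a one-second delay, reset on completion, repeatedly toggles the light's visibility.
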(event EventTick
  (params (DeltaSeconds :type Float%20%28single-precision%29))
  (bind _returnvalue (Game|GetPlayerCharacter 0))
  (bind _staticmeshcomponent0 (Variables|Default|GetStaticMeshComponent0))
  (bind _returnvalue_2 (Transformation|GetWorldLocation _staticmeshcomponent0))
  (bind _returnvalue_3 (Transformation|GetActorLocation _returnvalue))
  (bind _returnvalue_4 (Math|Rotator|FindLookatRotation _returnvalue_2 _returnvalue_3))
  (bind (_roll _pitch _yaw) (Math|Rotator|BreakRotator _returnvalue_4))
  (Utilities|FlowControl|Sequence
    (:then_0
      (Utilities|FlowControl|DoOnce false :!label _label
        (:Completed
          (Utilities|FlowControl|RetriggerableDelay (+ 0.0 1.0))
          (Rendering|ToggleVisibility (Variables|Default|GetPointLight) false)
          (goto _label Reset))))
    (:then_1
      (Transformation|SetWorldRotation (Variables|Default|GetStaticMeshComponent0) (Math|Rotator|MakeRotator 0.0 (+ _pitch 2.1e+02) (+ _yaw 9e+01)) false false))))

(fn ConstructionScript)