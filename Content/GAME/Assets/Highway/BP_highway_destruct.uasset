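; Highway destructible actor that fractures a bridge mesh when its trigger is overlapped, with smoke effects and a broken-bridge mesh.
; The overlap enables physics and applies huge damage and impulse along the player's forward vector.
; BeginPlay hides the broken bridge, then shows it and enables collision after a short delay.
; Both BeginPlay and overlap feed a shared delayed sequence that toggles two smoke effects and later destroys them and the fracture mesh.
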(event OnComponentBeginOverlap(Trigger)
  (params (OverlappedComponent :type Primitive%20Component%20Object%20Reference) (OtherActor :type Actor%20Object%20Reference) (OtherComp :type Primitive%20Component%20Object%20Reference) (OtherBodyIndex :type Integer) (bFromSweep :type Boolean) (SweepResult :type Hit%20Result%20Structure%20%28by%20ref%29))
  (bind _sm_highway_destrcutable_fracture_01_dm (Variables|Default|GetSM_Highway_destrcutable_Fracture_01_DM))
  (Physics|SetSimulatePhysics (Variables|Default|GetSM_Highway_destrcutable_Fracture_01_DM) true)
  (if true
    (Class|DestructibleComponent|ApplyDamage _sm_highway_destrcutable_fracture_01_dm 9999999999.0 (Transformation|GetWorldLocation _sm_highway_destrcutable_fracture_01_dm) (Transformation|GetActorForwardVector (Game|GetPlayerCharacter 0)) 1e+17)
    (Utilities|FlowControl|Sequence
      (:then_0
        (Utilities|FlowControl|Delay 1.8)
        (Components|Activation|ToggleActive (Variables|Default|GetPS_destructsmoke_1))
        (Utilities|FlowControl|Delay 13.0)
        (Components|DestroyComponent (Variables|Default|GetPS_destructsmoke_1)))
      (:then_1
        (Utilities|FlowControl|Delay 2.0)
        (Components|Activation|ToggleActive (Variables|Default|GetPS_destructsmoke))
        (Utilities|FlowControl|Delay 16.0)
        (Components|DestroyComponent (Variables|Default|GetPS_destructsmoke)))
      (:then_2
        (Utilities|FlowControl|Delay 5.0)
        (Components|DestroyComponent (Variables|Default|GetSM_Highway_destrcutable_Fracture_01_DM))))))

(event EventBeginPlay
  (Utilities|FlowControl|Sequence
    (:then_0
      (Rendering|SetVisibility (Variables|Default|GetSM_broken_bridge) false true)
      (Utilities|FlowControl|Delay 3.0)
      (Rendering|SetVisibility (Variables|Default|GetSM_broken_bridge) true true)
      (Collision|SetActorEnableCollision true))
    (:then_1
      (Components|Activation|Deactivate (Variables|Default|GetPS_destructsmoke_1))
      (Utilities|FlowControl|Sequence :!label _label
        (:then_0
          (Utilities|FlowControl|Delay 1.8)
          (Components|Activation|ToggleActive (Variables|Default|GetPS_destructsmoke_1))
          (Utilities|FlowControl|Delay 13.0)
          (Components|DestroyComponent (Variables|Default|GetPS_destructsmoke_1)))
        (:then_1
          (Utilities|FlowControl|Delay 2.0)
          (Components|Activation|ToggleActive (Variables|Default|GetPS_destructsmoke))
          (Utilities|FlowControl|Delay 16.0)
          (Components|DestroyComponent (Variables|Default|GetPS_destructsmoke)))
        (:then_2
          (Utilities|FlowControl|Delay 5.0)
          (Components|DestroyComponent (Variables|Default|GetSM_Highway_destrcutable_Fracture_01_DM)))))
    (:then_2
      (Components|Activation|Deactivate (Variables|Default|GetPS_destructsmoke))
      (goto _label))))

(fn ConstructionScript)