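; Flickering broken-glass bulb light that toggles its SpotLight and PointLight on and off at random intervals with a buzzing sound.
; Tick passes a DoOnce into a randomized retriggerable delay of just over a second, which flips both lights' visibility and resets the DoOnce to loop indefinitely.
; Each flip also plays the Lightbuzzing audio event at the actor's location.
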(event EventTick
  (params (DeltaSeconds :type Float%20%28single-precision%29))
  (Utilities|FlowControl|DoOnce false :!label _label
    (:Completed
      (Utilities|FlowControl|RetriggerableDelay (+ (Math|Random|RandomFloat) (* 1.0 1.3)))
      (Utilities|FlowControl|Sequence
        (:then_0
          (Rendering|ToggleVisibility (Variables|Default|GetSpotLight) false)
          (goto _label Reset))
        (:then_1
          (Class|FMODBlueprintStatics|PlayEventatLocation "/Game/FMOD/Events/Buildings/Lightbuzzing.Lightbuzzing" (Math|Conversions|ToTransform(Vector) (Transformation|GetActorLocation))))))))

(fn ConstructionScript)